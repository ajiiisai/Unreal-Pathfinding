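; BP_Grid is a tile grid actor that maps ground types from the world and previews paths between the selected and hovered tiles.
; Sphere traces on two channels fill StructTiles, using obstacle actors for terrain cost, with debug drawing at construction and BP_Tile actors spawned at BeginPlay.
; Hovering runs four-neighbor weighted A* with a Manhattan heuristic, stopping when the target is first reached, then highlights the retraced path.
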(event `self.ReceiveBeginPlay`
  (`KismetSystemLibrary.FlushPersistentDebugLines`)
  (set `self.GridLocation` (`SceneComponent.K2_GetComponentLocation` (`self.Scene`)))
  (`self.Generate Map Data from World`)
  (`self.SpawnTile` true))

(event `Event_NewTileSelected`
  (params (selectedTile :type "/Game/Art/Meshes/Grids/BP_Tile Object Reference"))
  (`/Engine/EditorBlueprintResources/StandardMacros.IsValid` (`self.selectedTile`)
    (:`Is Valid`
      (`/Game/Art/Meshes/Grids/BP_Tile.Event_DeselectTile` (`self.selectedTile`)))
    (:`Is Not Valid`
      _))
  (set `self.selectedTile` selectedTile))

(event `Event_NewTileOvered`
  (params (OveredTile :type "/Game/Art/Meshes/Grids/BP_Tile Object Reference"))
  (bind _overedtile (`self.overedTile`))
  (bind _selectedtile (`self.selectedTile`))
  (`/Engine/EditorBlueprintResources/StandardMacros.IsValid` (`self.overedTile`)
    (:`Is Valid`
      (`/Game/Art/Meshes/Grids/BP_Tile.Event_EndOverTile` (`self.overedTile`)))
    (:`Is Not Valid`
      _))
  (set `self.overedTile` OveredTile)
  (`self.HighlightCurrentPath` false)
  (if (and (`KismetSystemLibrary.IsValid` _selectedtile) (`KismetSystemLibrary.IsValid` _overedtile))
    (`self.FindPathToTarget` (`/Game/Art/Meshes/Grids/BP_Tile.GridIndex` _selectedtile) (`/Game/Art/Meshes/Grids/BP_Tile.GridIndex` _overedtile))
    (`self.HighlightCurrentPath` true)))

(fn `DrawTile`
  (locals (X :type Integer) (Y :type Integer) (TilePosition :type "Vector Structure"))
  (bind _keys (`BlueprintMapLibrary.Map_Keys` (`self.struct_Tiles`)))
  (for _array_element _keys
    (bind _value (`BlueprintMapLibrary.Map_Find` (`self.struct_Tiles`) _array_element))
    (`self.My Draw Debug Plane` (`.WorldLocation_5_BB7ACA274FE24577C85562BADC6DB6A7` (break `/Game/Blueprints/Grid/Struct_Tiles` _value)) (`.groundType_2_DEACFF2C4CF2A863598C36AB8530B466` (break `/Game/Blueprints/Grid/Struct_Tiles` _value)))))

(fn `FindPathToTarget`
  (params (startTile :type "Vector2D Structure") (targetTile :type "Vector2D Structure"))
  (locals (startTileL :type "Vector2D Structure") (targetTileL :type "Vector2D Structure") (openSet :type "Array of Vector2D Structure") (closedSet :type "Array of Vector2D Structure") (currentTile :type "Vector2D Structure") (openSetCheapest :type "Vector2D Structure") (currentNeighbour :type "Vector2D Structure") (currentNeighbourCostFromStart :type Integer))
  (bind _struct_tiles (`self.struct_Tiles`))
  (bind _struct_tiles_2 (`self.struct_Tiles`))
  (bind _struct_tiles_3 (`self.struct_Tiles`))
  (bind _currentneighbourcostfromstart (`local.currentNeighbourCostFromStart`))
  (bind _starttilel (`local.startTileL`))
  (bind _struct_tiles_4 (`self.struct_Tiles`))
  (bind _starttilel_2 (`local.startTileL`))
  (bind _value (`BlueprintMapLibrary.Map_Find` _struct_tiles _starttilel_2))
  (bind _value_2 (`BlueprintMapLibrary.Map_Find` _struct_tiles_3 (`local.currentNeighbour`)))
  (bind _costtotarget (`self.GetEstimatedCostToTarget` (`local.currentNeighbour`) (`local.targetTileL`)))
  (bind _costtotarget_2 (`self.GetEstimatedCostToTarget` (`local.startTileL`) (`local.targetTileL`)))
  (bind (_value_3 _returnvalue) (`BlueprintMapLibrary.Map_Find` (`self.struct_Tiles`) (`local.targetTileL`)))
  (bind _value_4 (`BlueprintMapLibrary.Map_Find` _struct_tiles_2 (`local.openSetCheapest`)))
  (set `local.startTileL` startTile)
  (set `local.targetTileL` targetTile)
  (if (and _returnvalue (`|EnumInequality` (`.groundType_2_DEACFF2C4CF2A863598C36AB8530B466` (break `/Game/Blueprints/Grid/Struct_Tiles` _value_3)) "NewEnumerator4") (`|EnumInequality` (`.groundType_2_DEACFF2C4CF2A863598C36AB8530B466` (break `/Game/Blueprints/Grid/Struct_Tiles` _value_3)) "NewEnumerator3"))
    (`|ExecutionSequence`
      (:`then_0`
        (bind _keys (`BlueprintMapLibrary.Map_Keys` (`self.struct_Tiles`)))
        (for _array_element _keys
          (bind _value_5 (`BlueprintMapLibrary.Map_Find` _struct_tiles_4 _array_element))
          (`BlueprintMapLibrary.Map_Add` _struct_tiles_4 _array_element (make `/Game/Blueprints/Grid/Struct_Tiles` (break `/Game/Blueprints/Grid/Struct_Tiles` _value_5) (`.groundType_2_DEACFF2C4CF2A863598C36AB8530B466` (break `/Game/Blueprints/Grid/Struct_Tiles` _value_5)) (`.WorldLocation_5_BB7ACA274FE24577C85562BADC6DB6A7` (break `/Game/Blueprints/Grid/Struct_Tiles` _value_5)) (`.GridIndex_8_08A2CD9C41211A8D181ABEAEC0668E0D` (break `/Game/Blueprints/Grid/Struct_Tiles` _value_5)) 999 (`.tileCost_18_899723B0490C87AF6A79E79D7DF03E07` (break `/Game/Blueprints/Grid/Struct_Tiles` _value_5)) 999 999)))
        (`BlueprintMapLibrary.Map_Add` _struct_tiles _starttilel_2 (make `/Game/Blueprints/Grid/Struct_Tiles` (break `/Game/Blueprints/Grid/Struct_Tiles` _value) (`.groundType_2_DEACFF2C4CF2A863598C36AB8530B466` (break `/Game/Blueprints/Grid/Struct_Tiles` _value)) (`.WorldLocation_5_BB7ACA274FE24577C85562BADC6DB6A7` (break `/Game/Blueprints/Grid/Struct_Tiles` _value)) (`.GridIndex_8_08A2CD9C41211A8D181ABEAEC0668E0D` (break `/Game/Blueprints/Grid/Struct_Tiles` _value)) _costtotarget_2 (`.tileCost_18_899723B0490C87AF6A79E79D7DF03E07` (break `/Game/Blueprints/Grid/Struct_Tiles` _value)) 0 _costtotarget_2)))
      (:`then_1`
        (set `local.currentTile` _starttilel)
        (`KismetArrayLibrary.Array_AddUnique` (`local.openSet`) _starttilel)
        (while (> (`KismetArrayLibrary.Array_Length` (`local.openSet`)) 0)
          (set `local.openSetCheapest` (`|GetArrayItem` (`local.openSet`)))
          (for _array_element_2 (`local.openSet`)
            (bind _value_6 (`BlueprintMapLibrary.Map_Find` _struct_tiles_2 _array_element_2))
            (if (< (`.finalCost_12_85BE75684B114E3C54A43A86389F36D5` (break `/Game/Blueprints/Grid/Struct_Tiles` _value_6)) (`.finalCost_12_85BE75684B114E3C54A43A86389F36D5` (break `/Game/Blueprints/Grid/Struct_Tiles` _value_4)))
              (set `local.openSetCheapest` _array_element_2 :!label _label)
              (elif (== (`.finalCost_12_85BE75684B114E3C54A43A86389F36D5` (break `/Game/Blueprints/Grid/Struct_Tiles` _value_6)) (`.finalCost_12_85BE75684B114E3C54A43A86389F36D5` (break `/Game/Blueprints/Grid/Struct_Tiles` _value_4)))
                (if (< (`.estimatedCostToTarget_19_66F89E444E3E004451EDF883FC11B9C8` (break `/Game/Blueprints/Grid/Struct_Tiles` _value_6)) (`.estimatedCostToTarget_19_66F89E444E3E004451EDF883FC11B9C8` (break `/Game/Blueprints/Grid/Struct_Tiles` _value_4)))
                  (goto _label)))))
          (set `local.currentTile` (`local.openSetCheapest`))
          (`KismetArrayLibrary.Array_RemoveItem` (`local.openSet`) (`local.currentTile`))
          (`KismetArrayLibrary.Array_AddUnique` (`local.closedSet`) (`local.currentTile`))
          (for _array_element_3 (`self.GetTileNeighbours` (`local.currentTile`))
            (set `local.currentNeighbour` _array_element_3)
            (if (not (`KismetArrayLibrary.Array_Contains` (`local.closedSet`) (`local.currentNeighbour`)))
              (set `local.currentNeighbourCostFromStart` (+ (`.costFromStart_14_9B33A7BC4B8C41A3A0E7669A70EA8D09` (break `/Game/Blueprints/Grid/Struct_Tiles` (`BlueprintMapLibrary.Map_Find` (`self.struct_Tiles`) (`local.currentTile`)))) (`.tileCost_18_899723B0490C87AF6A79E79D7DF03E07` (break `/Game/Blueprints/Grid/Struct_Tiles` (`BlueprintMapLibrary.Map_Find` (`self.struct_Tiles`) (`local.currentNeighbour`))))))
              (if (not (`KismetArrayLibrary.Array_Contains` (`local.openSet`) (`local.currentNeighbour`)))
                (`KismetArrayLibrary.Array_AddUnique` (`local.openSet`) (`local.currentNeighbour`))
                (`BlueprintMapLibrary.Map_Add` _struct_tiles_3 (`local.currentNeighbour`) (make `/Game/Blueprints/Grid/Struct_Tiles` (break `/Game/Blueprints/Grid/Struct_Tiles` _value_2) (`.groundType_2_DEACFF2C4CF2A863598C36AB8530B466` (break `/Game/Blueprints/Grid/Struct_Tiles` _value_2)) (`.WorldLocation_5_BB7ACA274FE24577C85562BADC6DB6A7` (break `/Game/Blueprints/Grid/Struct_Tiles` _value_2)) (`.GridIndex_8_08A2CD9C41211A8D181ABEAEC0668E0D` (break `/Game/Blueprints/Grid/Struct_Tiles` _value_2)) (+ _currentneighbourcostfromstart _costtotarget) (`.tileCost_18_899723B0490C87AF6A79E79D7DF03E07` (break `/Game/Blueprints/Grid/Struct_Tiles` _value_2)) _currentneighbourcostfromstart _costtotarget (`local.currentTile`)) :!label _label_2)
                (if (== (`local.currentNeighbour`) (`local.targetTileL`))
                  (set `self.path` (`self.RetracePath` (`local.targetTileL`) (`local.startTileL`)))
                  (return))
                (elif (< (`local.currentNeighbourCostFromStart`) (`.costFromStart_14_9B33A7BC4B8C41A3A0E7669A70EA8D09` (break `/Game/Blueprints/Grid/Struct_Tiles` _value_2)))
                  (goto _label_2))))))
        (return)))))

(fn `Generate Map Data from World`
  (locals (TilePosition :type "Vector Structure") (X :type Integer) (Y :type Integer))
  (bind (_gridtilenumberx _gridtilenumbery) (`self.GridTileNumber`))
  (bind _tilesize (`self.TileSize`))
  (bind _tilesize_2 (`self.TileSize`))
  (bind (_hitsomething _out_hit_hit_actor) (`self.MySphereTrace` (`local.TilePosition`) "TraceTypeQuery4"))
  (bind _returnvalue (`KismetMathLibrary.MakeVector2D` (`KismetMathLibrary.Conv_IntToDouble` (`local.X`)) (`KismetMathLibrary.Conv_IntToDouble` (`local.Y`))))
  (bind _returnvalue_2 (`KismetMathLibrary.MakeVector2D` (`KismetMathLibrary.Conv_IntToDouble` (`local.X`)) (`KismetMathLibrary.Conv_IntToDouble` (`local.Y`))))
  (bind _returnvalue_3 (`KismetMathLibrary.MakeVector2D` (`KismetMathLibrary.Conv_IntToDouble` (`local.X`)) (`KismetMathLibrary.Conv_IntToDouble` (`local.Y`))))
  (bind _enum_groundtypes (`/Game/Blueprints/Grid/BP_Base_Obstacle.Enum_GroundTypes` (cast `/Game/Blueprints/Grid/BP_Base_Obstacle` _out_hit_hit_actor :!pure true)))
  (for _index (range (+ _gridtilenumberx 1))
    (set `local.X` _index)
    (for _index_2 (range (+ _gridtilenumbery 1))
      (set `local.Y` _index_2)
      (set `local.TilePosition` (+ (`self.GridBottomLeft`) (* (`SceneComponent.GetRightVector` (`self.Scene`)) (+ (* (`local.X`) (* _tilesize_2 2.0)) _tilesize_2)) (* (`SceneComponent.GetForwardVector` (`self.Scene`)) (+ (* (`local.Y`) (* _tilesize 2.0)) _tilesize))))
      (if (`self.MySphereTrace` (`local.TilePosition`) "TraceTypeQuery3")
        (if _hitsomething
          (`BlueprintMapLibrary.Map_Add` (`self.struct_Tiles`) _returnvalue (make `/Game/Blueprints/Grid/Struct_Tiles` null _enum_groundtypes (`local.TilePosition`) _returnvalue 0 (`self.GetTileCost` _enum_groundtypes)))
          (else
            (`BlueprintMapLibrary.Map_Add` (`self.struct_Tiles`) _returnvalue_3 (make `/Game/Blueprints/Grid/Struct_Tiles` null "NewEnumerator0" (`local.TilePosition`) _returnvalue_3 0 (`self.GetTileCost` "NewEnumerator0")))))
        (else
          (`BlueprintMapLibrary.Map_Add` (`self.struct_Tiles`) _returnvalue_2 (make `/Game/Blueprints/Grid/Struct_Tiles` null "NewEnumerator4" (`local.TilePosition`) _returnvalue_2 0 (`self.GetTileCost` "NewEnumerator4"))))))))

(fn `GetEstimatedCostToTarget`
  (params (currentTile :type "Vector2D Structure") (targetTile :type "Vector2D Structure"))
  (returns (costToTarget :type Integer))
  (bind (_returnvalue_x _returnvalue_y) (`KismetMathLibrary.BreakVector2D` (- currentTile targetTile)))
  (return (`KismetMathLibrary.Round` (+ (`KismetMathLibrary.Abs` _returnvalue_x) (`KismetMathLibrary.Abs` _returnvalue_y)))))

(fn `GetTileCost`
  (params (gridIndex :type "/Game/Blueprints/Grid/Enum_GroundTypes Enum" :default "NewEnumerator0"))
  (returns (tileCost :type Integer))
  (locals (Cost :type Integer))
  (switch `/Game/Blueprints/Grid/Enum_GroundTypes` gridIndex
    (:`NewEnumerator0`
      (set `local.Cost` 1))
    (:`NewEnumerator1`
      (set `local.Cost` 2))
    (:`NewEnumerator2`
      (set `local.Cost` 5))
    (:`NewEnumerator3`
      (set `local.Cost` 999 :!label _label))
    (:`NewEnumerator4`
      (goto _label)))
  (return (`local.Cost`)))

(fn `GetTileNeighbours`
  (params (gridIndex :type "Vector2D Structure"))
  (returns (neighbours :type "Array of Vector2D Structure"))
  (locals (outNeighbours :type "Array of Vector2D Structure") (possibleNeighbours :type "Array of Vector2D Structure"))
  (bind _output_get (set `local.possibleNeighbours` (`|MakeArray` (1.0 0.0) (0.0 1.0) (-1.0 0.0) (0.0 -1.0) :!type "Vector2D Structure")))
  (for _array_element _output_get
    (bind _returnvalue (+ _array_element gridIndex))
    (bind (_value _returnvalue_2) (`BlueprintMapLibrary.Map_Find` (`self.struct_Tiles`) _returnvalue))
    (if _returnvalue_2
      (if (and (`|EnumInequality` (`.groundType_2_DEACFF2C4CF2A863598C36AB8530B466` (break `/Game/Blueprints/Grid/Struct_Tiles` _value)) "NewEnumerator4") (`|EnumInequality` (`.groundType_2_DEACFF2C4CF2A863598C36AB8530B466` (break `/Game/Blueprints/Grid/Struct_Tiles` _value)) "NewEnumerator3"))
        (`KismetArrayLibrary.Array_AddUnique` (`local.outNeighbours`) _returnvalue))))
  (return (`local.outNeighbours`)))

(fn `GridBottomLeft`
  (returns (GridBottomLeft :type "Vector Structure"))
  (bind (_gridsizeworld_x _gridsizeworld_y) (`KismetMathLibrary.BreakVector2D` (`self.GridSizeWorld`)))
  (bind _gridsizeworld_x_2 (`KismetMathLibrary.BreakVector2D` (`self.GridSizeWorld`)))
  (return (- (- (`self.GridLocation`) (* (`SceneComponent.GetRightVector` (`self.Scene`)) _gridsizeworld_x_2)) (* (`SceneComponent.GetForwardVector` (`self.Scene`)) _gridsizeworld_y))))

(fn `GridTileNumber`
  (returns (GridTileNumberX :type Integer) (GridTileNumberY :type Integer))
  (bind (_returnvalue_x _returnvalue_y) (`KismetMathLibrary.BreakVector2D` (/ (`self.GridSizeWorld`) (`self.TileSize`))))
  (return (- (`KismetMathLibrary.Round` _returnvalue_x) 1) (- (`KismetMathLibrary.Round` _returnvalue_y) 1)))

(fn `HighlightCurrentPath`
  (params (bIsForHighlight :type Boolean))
  (for _array_element (`self.path`)
    (bind _value (`BlueprintMapLibrary.Map_Find` (`self.struct_Tiles`) _array_element))
    (`/Engine/EditorBlueprintResources/StandardMacros.IsValid` (break `/Game/Blueprints/Grid/Struct_Tiles` _value)
      (:`Is Valid`
        (`/Game/Art/Meshes/Grids/BP_Tile.Event_IsInPath` (break `/Game/Blueprints/Grid/Struct_Tiles` _value) bIsForHighlight)))))

(fn `My Draw Debug Plane`
  (params (Location :type "Vector Structure") (GroundType :type "/Game/Blueprints/Grid/Enum_GroundTypes Enum" :default "NewEnumerator0"))
  (locals (TileColor :type "LinearColor Structure" :default (struct :`R` 1.0 :`G` 0.678676 :`A` 1.0)))
  (switch `/Game/Blueprints/Grid/Enum_GroundTypes` GroundType
    (:`NewEnumerator0`
      (set `local.TileColor` (struct :`R` 0.927995 :`G` 1.0 :`B` 0.869792 :`A` 1.0)))
    (:`NewEnumerator1`
      (set `local.TileColor` (struct :`R` 0.645192 :`G` 0.65625 :`B` 0.25293 :`A` 1.0)))
    (:`NewEnumerator2`
      (set `local.TileColor` (struct :`R` 0.369792 :`G` 0.137607 :`B` 0.048063 :`A` 1.0)))
    (:`NewEnumerator3`
      (set `local.TileColor` (struct :`R` 0.71875 :`G` 0.054792 :`A` 1.0))))
  (`KismetSystemLibrary.DrawDebugPlane` (make `Plane` (.z Location) 0.0 0.0 1.0) Location (- (`self.TileSize`) (`self.TileSizeMinus`)) (`local.TileColor`) 10000.0))

(fn `MySphereTrace`
  (params (Location :type "Vector Structure") (TraceChannel :type "ETraceTypeQuery Enum" :default "TraceTypeQuery1"))
  (returns (HitSomething :type Boolean) (`Out Hit Hit Actor` :type "Actor Object Reference"))
  (bind (_outhit _returnvalue) (`KismetSystemLibrary.SphereTraceSingle` Location Location (- (`self.TileSize`) (`self.TileSizeMinus`)) TraceChannel))
  (return _returnvalue (`.HitActor` (`GameplayStatics.BreakHitResult` _outhit))))

(fn `RetracePath`
  (params (targetTile :type "Vector2D Structure") (startTile :type "Vector2D Structure"))
  (returns (path :type "Array of Vector2D Structure"))
  (locals (currentTile :type "Vector2D Structure") (outPath :type "Array of Vector2D Structure") (invertedPath :type "Array of Vector2D Structure"))
  (set `local.currentTile` targetTile)
  (while (!= (`local.currentTile`) startTile)
    (`KismetArrayLibrary.Array_AddUnique` (`local.invertedPath`) (`local.currentTile`))
    (set `local.currentTile` (`.previousTile_25_649E552445DA543EC30E1896C59EE6AF` (break `/Game/Blueprints/Grid/Struct_Tiles` (`BlueprintMapLibrary.Map_Find` (`self.struct_Tiles`) (`local.currentTile`))))))
  (bind (_arrayindex _arrayelement) (`/Engine/EditorBlueprintResources/StandardMacros.ReverseForEachLoop` (`local.invertedPath`))
    (:`LoopBody`
      (`KismetArrayLibrary.Array_AddUnique` (`local.outPath`) _arrayelement))
    (:`Completed`
      (return (`local.outPath`)))))

(fn `SpawnTile`
  (params (bSpawnNoneTile :type Boolean))
  (bind _struct_tiles (`self.struct_Tiles`))
  (bind _keys (`BlueprintMapLibrary.Map_Keys` (`self.struct_Tiles`)))
  (for _array_element _keys
    (bind _value (`BlueprintMapLibrary.Map_Find` _struct_tiles _array_element))
    (if (or (`|EnumInequality` (`.groundType_2_DEACFF2C4CF2A863598C36AB8530B466` (break `/Game/Blueprints/Grid/Struct_Tiles` _value)) "NewEnumerator4") bSpawnNoneTile)
      (bind _returnvalue (`|SpawnActorFromClass` "/Game/Art/Meshes/Grids/BP_Tile.BP_Tile_C" (`KismetMathLibrary.Conv_VectorToTransform` (`.WorldLocation_5_BB7ACA274FE24577C85562BADC6DB6A7` (break `/Game/Blueprints/Grid/Struct_Tiles` _value))) "Undefined" "MultiplyWithRoot" null self null))
      (set `/Game/Art/Meshes/Grids/BP_Tile.GridIndex` _array_element _returnvalue)
      (`BlueprintMapLibrary.Map_Add` _struct_tiles _array_element (make `/Game/Blueprints/Grid/Struct_Tiles` _returnvalue (`.groundType_2_DEACFF2C4CF2A863598C36AB8530B466` (break `/Game/Blueprints/Grid/Struct_Tiles` _value)) (`.WorldLocation_5_BB7ACA274FE24577C85562BADC6DB6A7` (break `/Game/Blueprints/Grid/Struct_Tiles` _value)) (`.GridIndex_8_08A2CD9C41211A8D181ABEAEC0668E0D` (break `/Game/Blueprints/Grid/Struct_Tiles` _value)) (`.finalCost_12_85BE75684B114E3C54A43A86389F36D5` (break `/Game/Blueprints/Grid/Struct_Tiles` _value)) (`.tileCost_18_899723B0490C87AF6A79E79D7DF03E07` (break `/Game/Blueprints/Grid/Struct_Tiles` _value)) (`.costFromStart_14_9B33A7BC4B8C41A3A0E7669A70EA8D09` (break `/Game/Blueprints/Grid/Struct_Tiles` _value)) (`.estimatedCostToTarget_19_66F89E444E3E004451EDF883FC11B9C8` (break `/Game/Blueprints/Grid/Struct_Tiles` _value)) (`.previousTile_25_649E552445DA543EC30E1896C59EE6AF` (break `/Game/Blueprints/Grid/Struct_Tiles` _value)))))))

(fn `UserConstructionScript`
  (bind (_gridsizeworld_x _gridsizeworld_y) (`KismetMathLibrary.BreakVector2D` (`self.GridSizeWorld`)))
  (`KismetSystemLibrary.FlushPersistentDebugLines`)
  (set `self.GridLocation` (`SceneComponent.K2_GetComponentLocation` (`self.Scene`)))
  (`KismetSystemLibrary.DrawDebugBox` (`self.GridLocation`) (`KismetMathLibrary.MakeVector` _gridsizeworld_y _gridsizeworld_x 5.0) (`self.GridBoxColor`) (struct) 100000.0 10.0)
  (`KismetSystemLibrary.DrawDebugBox` (`self.GridBottomLeft`) (20.0 20.0 20.0) (`self.BottomLeftColor`) (struct) 100000.0 10.0)
  (`self.Generate Map Data from World`)
  (`self.DrawTile`))