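; BP_Tile is a clickable grid tile whose color shows its ground type and its hover, selection and path state.
; It reports hover and click to BPGrid and exposes events to end hover, deselect or mark it as in path.
; SetTileColor reads tile data from the grid by GridIndex, then layers hover brightening, path override and selection flag into material parameters.
; A W_GridTile widget receives the grid and index after a one-tick delay.
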(event `self.ReceiveBeginPlay`
  (`KismetSystemLibrary.DelayUntilNextTick`)
  (`self.SetTileColor`)
  (`self.SetWidgetVariables`))

(event `self.StaticMesh.OnBeginCursorOver`
  (params (TouchedComponent :type "PrimitiveComponent Object Reference"))
  (`self.Event_StartOverTile`)
  (`/Game/Blueprints/Grid/BP_Grid.Event_NewTileOvered` (`self.BP_Grid`) self))

(event `Event_StartOverTile`
  (set `self.bIsOvered` true)
  (`self.SetTileColor` :!label _label))

(event `self.StaticMesh.OnEndCursorOver`
  (params (TouchedComponent :type "PrimitiveComponent Object Reference")))

(event `Event_EndOverTile`
  (set `self.bIsOvered` false)
  (goto _label))

(event `self.StaticMesh.OnClicked`
  (params (TouchedComponent :type "PrimitiveComponent Object Reference") (ButtonPressed :type "Key Structure"))
  (`self.Event_SelectTile`)
  (`/Game/Blueprints/Grid/BP_Grid.Event_NewTileSelected` (`self.BP_Grid`) self))

(event `Event_SelectTile`
  (set `self.bIsSelected` true)
  (`self.SetTileColor` :!label _label_2))

(event `Event_DeselectTile`
  (set `self.bIsSelected` false)
  (goto _label_2))

(event `Event_IsInPath`
  (params (bIsInPath :type Boolean))
  (set `self.bIsInPath` bIsInPath)
  (`self.SetTileColor`))

(fn `GetTileData`
  (returns (Value :type "/Game/Blueprints/Grid/Struct_Tiles Structure"))
  (return (`BlueprintMapLibrary.Map_Find` (`/Game/Blueprints/Grid/BP_Grid.struct_Tiles` (`self.BP_Grid`)) (`self.GridIndex`))))

(fn `SetTileColor`
  (locals (tileColor :type "LinearColor Structure"))
  (bind (_value_tileactor _value_groundtype) (break `/Game/Blueprints/Grid/Struct_Tiles` (`self.GetTileData`)))
  (`|ExecutionSequence`
    (:`then_0`
      (switch `/Game/Blueprints/Grid/Enum_GroundTypes` _value_groundtype
        (:`NewEnumerator0`
          (set `local.TileColor` (struct :`R` 0.115999 :`G` 0.125 :`B` 0.108724 :`A` 1.0)))
        (:`NewEnumerator1`
          (set `local.TileColor` (struct :`R` 0.645192 :`G` 0.65625 :`B` 0.25293 :`A` 1.0)))
        (:`NewEnumerator2`
          (set `local.TileColor` (struct :`R` 0.369792 :`G` 0.137607 :`B` 0.048063 :`A` 1.0)))
        (:`NewEnumerator3`
          (set `local.TileColor` (struct :`R` 0.71875 :`G` 0.054792 :`A` 1.0)))
        (:`NewEnumerator4`
          (set `local.TileColor` (struct :`R` 0.046875 :`G` 0.044745 :`B` 0.040039 :`A` 1.0)))))
    (:`then_1`
      (if (`self.bIsSelected`)
        (`MeshComponent.SetScalarParameterValueOnMaterials` (`self.StaticMesh`) "bIsSelected" 1.0)
        (else
          (`MeshComponent.SetScalarParameterValueOnMaterials` (`self.StaticMesh`) "bIsSelected" 0.0))))
    (:`then_2`
      (if (`self.bIsOvered`)
        (set `local.tileColor` (`KismetMathLibrary.Conv_VectorToLinearColor` (* (`KismetMathLibrary.Conv_LinearColorToVector` (`local.tileColor`)) 3.0)))))
    (:`then_3`
      (if (`self.bIsInPath`)
        (set `local.tileColor` (struct :`G` 0.43094 :`B` 1.0 :`A` 1.0))))
    (:`then_4`
      (`MeshComponent.SetVectorParameterValueOnMaterials` (`self.StaticMesh`) "Color" (`KismetMathLibrary.Conv_LinearColorToVector` (`local.tileColor`))))))

(fn `SetTileSize`
  (bind _staticmesh (`self.StaticMesh`))
  (bind (_returnvalue_x _returnvalue_y _returnvalue_z) (`KismetMathLibrary.BreakVector` (* (`SceneComponent.K2_GetComponentScale` _staticmesh) (/ (`/Game/Blueprints/Grid/BP_Grid.TileSize` (`self.BP_Grid`)) 50.0))))
  (`SceneComponent.SetWorldScale3D` _staticmesh (`KismetMathLibrary.MakeVector` _returnvalue_x _returnvalue_y _returnvalue_z)))

(fn `SetWidgetVariables`
  (bind _asw_grid_tile (cast `/Game/Blueprints/Grid/W_GridTile` (`WidgetComponent.GetUserWidgetObject` (`self.Widget`)) :!pure true))
  (set `/Game/Blueprints/Grid/W_GridTile.grid` (`self.BP_Grid`) _asw_grid_tile)
  (set `/Game/Blueprints/Grid/W_GridTile.gridIndex` (`self.GridIndex`) _asw_grid_tile))

(fn `UserConstructionScript`)